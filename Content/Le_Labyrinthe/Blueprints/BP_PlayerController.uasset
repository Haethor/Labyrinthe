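; Player controller for the first-person character in Le Labyrinthe, turning Enhanced Input actions into character control.
; BeginPlay registers the player mapping context on the local player subsystem.
; Input events drive crouch, jump, control-rotation-relative movement and mouse look, with movement also toggling an IsWalking flag.
; The Use action fires a forward line trace on the Camera channel, but its result is not yet used.
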(event `self.ReceiveBeginPlay`
  (bind _returnvalue (subsystem `EnhancedInputLocalPlayerSubsystem`))
  ;[1 1 1] Comment
  (`/Engine/EditorBlueprintResources/StandardMacros.IsValid` _returnvalue
    (:`Is Valid`
      (`EnhancedInputSubsystemInterface.AddMappingContext` _returnvalue "/Game/Le_Labyrinthe/Inputs/IMC_Player.IMC_Player" 0 (struct))
      (`EnhancedInputSubsystemInterface.AddMappingContext` _returnvalue null 0 (struct))
      (cast `/Game/Le_Labyrinthe/Blueprints/BP_FirstPersonCharacter` (`GameplayStatics.GetPlayerCharacter` 0)))))

(event `EnhancedInput|/Game/Le_Labyrinthe/Inputs/IA_Crouch`
  (params (ActionValue :type Boolean) (ElapsedSeconds :type "Float (double-precision)") (TriggeredSeconds :type "Float (double-precision)") (InputAction :type "InputAction Object Reference" :default "/Game/Le_Labyrinthe/Inputs/IA_Crouch.IA_Crouch"))
  (bind _returnvalue (`GameplayStatics.GetPlayerCharacter` 0))
  ;[1 1 1] Movement
  (:`Started`
    (`Character.Crouch` _returnvalue))
  (:`Completed`
    (`Character.UnCrouch` _returnvalue)))

(event `EnhancedInput|/Game/Le_Labyrinthe/Inputs/IA_Jump`
  (params (ActionValue :type Boolean) (ElapsedSeconds :type "Float (double-precision)") (TriggeredSeconds :type "Float (double-precision)") (InputAction :type "InputAction Object Reference" :default "/Game/Le_Labyrinthe/Inputs/IA_Jump.IA_Jump"))
  (bind _returnvalue (`GameplayStatics.GetPlayerCharacter` 0))
  ;[1 1 1] Movement
  (:`Started`
    (`Character.Jump` _returnvalue))
  (:`Completed`
    (`Character.StopJumping` _returnvalue)))

(event `EnhancedInput|/Game/Le_Labyrinthe/Inputs/IA_Move`
  (params (ActionValue :type "Vector2D Structure") (ElapsedSeconds :type "Float (double-precision)") (TriggeredSeconds :type "Float (double-precision)") (InputAction :type "InputAction Object Reference" :default "/Game/Le_Labyrinthe/Inputs/IA_Move.IA_Move"))
  (bind (_returnvalue_roll _returnvalue_pitch _returnvalue_yaw) (`KismetMathLibrary.BreakRotator` (`self.GetControlRotation`)))
  (bind _returnvalue (`GameplayStatics.GetPlayerCharacter` 0))
  ;[1 1 1] Movement
  (:`Triggered`
    (`Pawn.AddMovementInput` _returnvalue (`KismetMathLibrary.GetRightVector` (`KismetMathLibrary.MakeRotator` _returnvalue_roll 0.0 _returnvalue_yaw)) ActionValue_X false)
    (`Pawn.AddMovementInput` _returnvalue (`KismetMathLibrary.GetForwardVector` (`KismetMathLibrary.MakeRotator` 0.0 0.0 _returnvalue_yaw)) ActionValue_Y false)
    (set `self.isWalking` true))
  (:`Completed`
    (set `self.isWalking` false)))

(event `EnhancedInput|/Game/Le_Labyrinthe/Inputs/IA_Mouse`
  (params (ActionValue :type "Vector2D Structure") (ElapsedSeconds :type "Float (double-precision)") (TriggeredSeconds :type "Float (double-precision)") (InputAction :type "InputAction Object Reference" :default "/Game/Le_Labyrinthe/Inputs/IA_Mouse.IA_Mouse"))
  (:`Triggered`
    (`self.AddYawInput` ActionValue_X)
    (`self.AddPitchInput` ActionValue_Y)))

(event `EnhancedInput|/Game/Le_Labyrinthe/Inputs/IA_Use`
  (params (ActionValue :type Boolean) (ElapsedSeconds :type "Float (double-precision)") (TriggeredSeconds :type "Float (double-precision)") (InputAction :type "InputAction Object Reference" :default "/Game/Le_Labyrinthe/Inputs/IA_Use.IA_Use"))
  (bind _returnvalue (`SceneComponent.K2_GetComponentLocation`))
  (:`Triggered`
    (`KismetSystemLibrary.LineTraceSingle` :`Start` _returnvalue :`End` (+ _returnvalue (* (`KismetMathLibrary.GetForwardVector` (`SceneComponent.K2_GetComponentRotation`)) (`KismetMathLibrary.Conv_DoubleToVector` 1500.0))) :`TraceChannel` "TraceTypeQuery2" :`DrawTime` 2.0)))

(fn `UserConstructionScript`)